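; An explosive barrel gravity target that detonates when its health runs out or when a throw ends.
; The TakeDamage event subtracts from Health and calls Explode at zero or below, while the OnThrowEnd override runs the parent logic and then explodes.
; Explode uses an IsAlive guard to fire once, spawning BP_Explosion at the Visual component's location with the barrel's damage and radius, then destroying the actor.
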(event `/Game/Interfaces/IDestructible.TakeDamage`
  (params (Dmage :type "Float (single-precision)"))
  (`self.TakeDamage_Internal` Dmage))

(fn `Explode`
  (if (`self.bIsAlive`)
    (set `self.bIsAlive` false)
    (`|SpawnActorFromClass` "/Game/LDIs/GravityTargets/BP_Explosion.BP_Explosion_C" (`KismetMathLibrary.MakeTransform` (`SceneComponent.K2_GetComponentLocation` (`self.Visual`))) "AlwaysSpawn" "OverrideRootScale" null (`self.ExplosionDamage`) (`self.ExplosionRadius`) null)
    (`self.K2_DestroyActor`)))

(fn `OnThrowEnd`
  (params (Hit :type "HitResult Structure"))
  (`parent.OnThrowEnd` Hit)
  (`self.Explode`))

(fn `TakeDamage_Internal`
  (params (Damage :type "Float (double-precision)"))
  (bind _output_get (set `self.Health` (- (`self.Health`) Damage)))
  (if (and (<= _output_get 0.0) (`self.bIsAlive`))
    (`self.Explode`)))

(fn `UserConstructionScript`
  (`parent.UserConstructionScript`))