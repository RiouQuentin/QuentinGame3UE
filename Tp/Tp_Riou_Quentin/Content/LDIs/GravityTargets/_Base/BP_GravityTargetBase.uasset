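; Base actor for gravity targets that can be grabbed, dropped or thrown, driven by a state machine (Idle, Grab Travel, Grabbed, Throw).
; Grabbing disables physics, swaps scale and collision profile, attaches to the grab point and lerps there on Tick.
; Dropping or throwing detaches, restores scale and physics, with throws adding an impulse.
; The first hit during a throw moves the actor to its simulated Visual and returns to Idle.
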(event `self.ReceiveBeginPlay`
  (`self.InTarget`))

(event `self.ReceiveTick`
  (params (DeltaSeconds :type "Float (single-precision)"))
  (switch `/Game/LDIs/GravityTargets/_Enums/EGravityTragetState` (`self.CurrentState`)
    (:`NewEnumerator1`
      (`self.UpdateGrabTravel` DeltaSeconds))))

(event `self.Visual.OnComponentHit`
  (params (HitComponent :type "PrimitiveComponent Object Reference") (OtherActor :type "Actor Object Reference") (OtherComp :type "PrimitiveComponent Object Reference") (NormalImpulse :type "Vector Structure") (Hit :type "HitResult Structure (by ref)"))
  (if (`|EnumEquality` (`self.CurrentState`) "NewEnumerator3")
    (`self.OnThrowEnd`)))

(fn `ActivatePhisics`
  (params (bActive :type Boolean))
  (locals (L_colProfileDefault :type Name :default "GravityGunObject") (L_colProfileGrab :type Name :default "OverlapAllDynamic"))
  (bind _visual (`self.Visual`))
  (`|ExecutionSequence`
    (:`then_0`
      (`PrimitiveComponent.SetSimulatePhysics` _visual bActive))
    (:`then_1`
      (`PrimitiveComponent.SetEnableGravity` _visual bActive))
    (:`then_2`
      (if bActive
        (`PrimitiveComponent.SetCollisionProfileName` _visual (`local.L_colProfileDefault`) true)
        (else
          (`PrimitiveComponent.SetCollisionProfileName` _visual (`local.L_colProfileGrab`) true))))
    (:`then_3`
      (`SceneComponent.K2_AttachToComponent` _visual (`self.DefaultSceneRoot`) "None" "SnapToTarget" "SnapToTarget" "SnapToTarget" true))
    (:`then_4`
      (`SceneComponent.K2_SetRelativeLocationAndRotation` :`self` _visual :`NewLocation` (0.0 0.1 0.0)))))

(fn `InTarget`
  (bind _visual (`self.Visual`))
  (`|ExecutionSequence`
    (:`then_0`
      (set `self.GrabFinalLocation` null))
    (:`then_1`
      (set `self.GrabTravelPercent` 0.0))
    (:`then_2`
      (set `self.ScaleDefault` (`SceneComponent.K2_GetComponentScale` _visual)))
    (:`then_3`
      (`PrimitiveComponent.SetMassOverrideInKg` _visual "None" 1.0 true))
    (:`then_4`
      (`self.SetState` "NewEnumerator0"))))

(fn `OnDropped`
  (`|ExecutionSequence`
    (:`then_0`
      (`KismetSystemLibrary.PrintString` (`KismetStringLibrary.Concat_StrStr` (`KismetSystemLibrary.GetDisplayName` self) "DROP") true true (struct :`R` 1.0 :`B` 0.058392 :`A` 1.0)))
    (:`then_1`
      (`self.ResetActor`))
    (:`then_2`
      (`self.ActivatePhisics` true))
    (:`then_3`
      (`self.SetState` "NewEnumerator0"))))

(fn `OnGrabbed`
  (params (GrabLocation :type "SceneComponent Object Reference"))
  (`|ExecutionSequence`
    (:`then_0`
      (`KismetSystemLibrary.PrintString` (`KismetStringLibrary.Concat_StrStr` (`KismetSystemLibrary.GetDisplayName` self) "GRABBED")))
    (:`then_1`
      (set `self.GrabFinalLocation` GrabLocation))
    (:`then_2`
      (`self.SetState` "NewEnumerator1"))))

(fn `OnGrabTravelEnd`
  (set `self.GrabTravelPercent` 0.0))

(fn `OnGrabTravelStart`
  (`|ExecutionSequence`
    (:`then_0`
      (`self.ActivatePhisics` false))
    (:`then_1`
      (`SceneComponent.SetWorldScale3D` (`self.Visual`) (`self.ScaleGrabbed`)))
    (:`then_2`
      (`self.K2_AttachToComponent` self (`self.GrabFinalLocation`) "None" "KeepWorld" "KeepWorld" "KeepWorld" true))
    (:`then_3`
      (set `self.GrabTravelPercent` 0.0))))

(fn `OnThrowEnd`
  (bind _visual (`self.Visual`))
  (bind (_returnvalue_location _returnvalue_rotation) (`KismetMathLibrary.BreakTransform` (`SceneComponent.K2_GetComponentToWorld` _visual)))
  (`|ExecutionSequence`
    (:`then_0`
      (`SceneComponent.K2_DetachFromComponent` _visual "KeepRelative" "KeepRelative" "KeepRelative" true))
    (:`then_1`
      (`self.K2_SetActorLocationAndRotation` self _returnvalue_location _returnvalue_rotation false false))
    (:`then_2`
      (`SceneComponent.K2_AttachToComponent` _visual (`self.DefaultSceneRoot`) "None" "KeepRelative" "KeepRelative" "KeepRelative" true))
    (:`then_3`
      (`self.SetState` "NewEnumerator0"))))

(fn `OnThrown`
  (params (ThrowVector :type "Vector Structure"))
  (set `self.ThrowVector` ThrowVector)
  (`|ExecutionSequence`
    (:`then_0`
      (`KismetSystemLibrary.PrintString` (`KismetStringLibrary.Concat_StrStr` (`KismetSystemLibrary.GetDisplayName` self) "THROW") true true (struct :`G` 1.0 :`B` 0.030708 :`A` 1.0)))
    (:`then_1`
      (`self.SetState` "NewEnumerator3"))))

(fn `OnThrowStart`
  (`|ExecutionSequence`
    (:`then_0`
      (`self.ResetActor`))
    (:`then_1`
      (`self.ActivatePhisics` true))
    (:`then_2`
      (`PrimitiveComponent.AddImpulse` (`self.Visual`) (`self.ThrowVector`) "None" false))))

(fn `ResetActor`
  (`|ExecutionSequence`
    (:`then_0`
      (`self.K2_DetachFromActor` "KeepWorld" "KeepWorld" "KeepWorld"))
    (:`then_1`
      (set `self.GrabFinalLocation` null))
    (:`then_2`
      (`SceneComponent.SetWorldScale3D` (`self.Visual`) (`self.ScaleDefault`)))))

(fn `SetState`
  (params (NewState :type "/Game/LDIs/GravityTargets/_Enums/EGravityTragetState Enum" :default "NewEnumerator0"))
  (bind _output_get (set `self.CurrentState` NewState))
  (switch `/Game/LDIs/GravityTargets/_Enums/EGravityTragetState` _output_get
    (:`NewEnumerator1`
      (`self.OnGrabTravelStart`))
    (:`NewEnumerator2`
      (`self.OnGrabTravelEnd`))
    (:`NewEnumerator3`
      (`self.OnThrowStart`))))

(fn `UpdateGrabTravel`
  (params (DeltaTime :type "Float (double-precision)"))
  (bind (_returnvalue_location _returnvalue_rotation) (`KismetMathLibrary.BreakTransform` (`KismetMathLibrary.TLerp` (`self.GetTransform`) (`SceneComponent.K2_GetComponentToWorld` (`self.GrabFinalLocation`)) (`self.GrabTravelPercent`))))
  (set `self.GrabTravelPercent` (+ (* DeltaTime (`self.GrabTravelSpeed`)) (`self.GrabTravelPercent`)))
  (`|ExecutionSequence`
    (:`then_0`
      (`self.K2_SetActorLocationAndRotation` _returnvalue_location _returnvalue_rotation false true))
    (:`then_1`
      (if (>= (`self.GrabTravelPercent`) 1.0)
        (`self.SetState` "NewEnumerator2")))))

(fn `UserConstructionScript`)