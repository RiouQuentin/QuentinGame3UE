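; BP_Door is a locked door actor that a player holding a key opens.
; Each tick, while PlayerInTrigger is valid, it checks for a key, removes one, shows VisualKey and sets MustOpen.
; The following tick latches IsOpen, waits DelayBeforeOpen, then calls OpenDoor, which simply destroys the actor.
; PlayerInTrigger is only read here, never assigned.
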(event `self.ReceiveBeginPlay`
  (`|ExecutionSequence`
    (:`then_0`
      (set `self.bMustOpen` false))
    (:`then_1`
      (set `self.bIsOpen` false))))

(event `self.ReceiveTick`
  (params (DeltaSeconds :type "Float (single-precision)"))
  (if (`self.bMustOpen`)
    (set `self.bMustOpen` false)
    (if (not (`self.bIsOpen`))
      (set `self.bIsOpen` true)
      (`KismetSystemLibrary.Delay` (`self.DelayBeforeOpen`))
      (`self.OpenDoor`))
    (else
      (`self.PlayerInTrigger`
        (:`then`
          (`self.CheckOpenDoor`))
        (:`else`)))))

(fn `CheckOpenDoor`
  (bind _playerintrigger (`self.PlayerInTrigger`))
  (if (`/Game/Player/BP_Player.HasKey` _playerintrigger)
    (`/Game/Player/BP_Player.RemoveKeys` _playerintrigger 1)
    (set `self.bMustOpen` true)
    (`SceneComponent.SetVisibility` (`self.Visual_Key`) true false)))

(fn `OpenDoor`
  (`self.K2_DestroyActor`))

(fn `UserConstructionScript`
  (`parent.UserConstructionScript`))