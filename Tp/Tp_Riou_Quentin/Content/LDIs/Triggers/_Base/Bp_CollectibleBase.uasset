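; Base collectible trigger Blueprint that grants a key to the player standing inside it.
; Each Tick it checks for a valid PlayerInTrigger while CanCollect is set, then calls CollectKey.
; CollectKey adds one key to the player, clears CanCollect and destroys the actor.
; The construction script only runs the parent's, and overlap tracking is not defined in this graph.
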(event `self.ReceiveTick`
  (params (DeltaSeconds :type "Float (single-precision)"))
  (`self.PlayerInTrigger`
    (:`then`
      (if (`self.bCanCollect`)
        (`self.CollectKey`)))
    (:`else`)))

(fn `CollectKey`
  (`/Game/Player/BP_Player.AddKeys` (`self.PlayerInTrigger`) 1)
  (set `self.bCanCollect` false)
  (`self.K2_DestroyActor`))

(fn `UserConstructionScript`
  (`parent.UserConstructionScript`))