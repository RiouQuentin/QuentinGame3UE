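; Base trigger Blueprint that tracks the BP_Player currently inside it.
; It extends the parent trigger's enter and leave handlers, storing any entering actor that casts to BP_Player in PlayerInTrigger.
; The reference clears only when that same actor leaves, so it holds a single player at a time and other actors do not affect it.
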(fn `OnActorTriggerEnter`
  (params (Actor :type "Actor Object Reference"))
  (`parent.OnActorTriggerEnter` Actor)
  (bind _asbp_player (cast `/Game/Player/BP_Player` Actor))
  (set `self.PlayerInTrigger` _asbp_player))

(fn `OnActorTriggerLeave`
  (params (Actor :type "Actor Object Reference"))
  (`parent.OnActorTriggerLeave` null)
  (if (== Actor (`self.PlayerInTrigger`))
    (set `self.PlayerInTrigger` null)))

(fn `UserConstructionScript`
  (`parent.UserConstructionScript`))