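; BP_HealthZone is a trigger zone that either damages or heals the player, chosen by the IsDammage flag.
; The construction script calls its parent, then gives the Visual component a damage or heal material to match.
; On Tick, while PlayerInTrigger is valid, it applies the per-second rate scaled by delta time through TakeDamage or AddHealth.
; PlayerInTrigger is only read here, not assigned.
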(event `self.ReceiveTick`
  (params (DeltaSeconds :type "Float (single-precision)"))
  (`self.PlayerInTrigger`
    (:`then`
      (`self.ApplyZoneEffect` DeltaSeconds))
    (:`else`)))

(fn `ApplyZoneEffect`
  (params (DeltaTime :type "Float (double-precision)"))
  (bind _playerintrigger (`self.PlayerInTrigger`))
  (bind _l_deltatime (`self.L_DeltaTime`))
  (set `self.L_DeltaTime` DeltaTime)
  (if (`self.bIsDammage`)
    (`/Game/Interfaces/IDestructible.TakeDamage` _playerintrigger (* (`self.DamagePerSecond`) _l_deltatime))
    (else
      (`/Game/Player/BP_Player.AddHealth` _playerintrigger (* _l_deltatime (`self.HealthPerSecond`))))))

(fn `UserConstructionScript`
  (locals (L_material :type "Material Object Reference"))
  (`parent.UserConstructionScript`)
  (if (`self.bIsDammage`)
    (set `local.L_material` (`self.MatDammage`))
    (else
      (set `local.L_material` (`self.MatHeal`))))
  (`PrimitiveComponent.SetMaterial` (`self.Visual`) 0 (`local.L_material`)))