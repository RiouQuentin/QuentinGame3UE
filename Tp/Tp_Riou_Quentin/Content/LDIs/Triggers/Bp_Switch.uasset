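; Switch trigger Blueprint that shows an on or off material and fires a linked Action.
; Tick sets the Interaction flag from whether PlayerInTrigger is valid, and the OnInteraction event can also set it.
; Both paths run InterationInternal, which swaps the mesh material and calls Switch on Action when the flag is true.
; Because this runs from Tick, Switch repeats every frame while PlayerInTrigger stays valid.
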(event `self.ReceiveTick`
  (params (DeltaSeconds :type "Float (single-precision)"))
  (`self.PlayerInTrigger`
    (:`then`
      (set `self.Interaction` true))
    (:`else`
      (set `self.Interaction` false)))
  (`self.Interation_Internal`))

(event `/Game/Interfaces/IInteractible.OnInteraction`
  (params (Interaction :type Boolean))
  (set `self.Interaction` Interaction)
  (`self.Interation_Internal`))

(fn `Interation_Internal`
  (locals (L_Material :type "Material Object Reference"))
  (if (`self.Interaction`)
    (set `local.L_Material` (`self.On`))
    (else
      (set `local.L_Material` (`self.Off`))))
  (`PrimitiveComponent.SetMaterial` (`self.Statick Mesh`) 0 (`local.L_Material`))
  (if (`self.Interaction`)
    (`/Game/LDIs/Triggers/BP_Door.Switch` (`self.Action`))))

(fn `UserConstructionScript`
  (`parent.UserConstructionScript`))