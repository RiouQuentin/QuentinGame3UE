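; Player controller that turns movement, aim and jump input into commands on the controlled BP_Player pawn.
; Input events cache axis values and jump state, and Tick dispatches to Idle, Moving or Jumping handlers based on the state read from the pawn.
; Handlers switch states and call the pawn's movement (scaled by delta time), aiming and jump functions.
; Landing detection appears intended to use near-zero vertical velocity.
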(event `InputAction|Jump`
  (params (Key :type "Key Structure"))
  (:`Pressed`
    (set `self.bJumpPressed` true))
  (:`Released`
    (set `self.bJumpPressed` false)))

(event `self.ReceiveBeginPlay`
  (`self.InitController`))

(event `self.ReceiveTick`
  (params (DeltaSeconds :type "Float (single-precision)"))
  (set `self.DeltaTime` DeltaSeconds)
  (`self.UpdateInput`))

(event `InputAxis|Move_Right`
  (params (AxisValue :type "Float (single-precision)"))
  (set `self.MvtRight` AxisValue))

(event `InputAxis|Move_Forward`
  (params (AxisValue :type "Float (single-precision)"))
  (set `self.MvtForward` AxisValue))

(event `InputAxis|Aim_Vertical`
  (params (AxisValue :type "Float (single-precision)"))
  (set `self.AimVertical` AxisValue))

(event `InputAxis|Aim_Horizontal`
  (params (AxisValue :type "Float (single-precision)"))
  (set `self.AimHorizontal` AxisValue))

(fn `InitController`
  (`|ExecutionSequence`
    (:`then_0`
      (bind _asbp_player (cast `/Game/Player/BP_Player` (`self.K2_GetPawn`)))
      (set `self.PlayerRef` _asbp_player))
    (:`then_1`
      (`/Game/Player/BP_Player.SetState` (`self.PlayerRef`) "NewEnumerator0"))
    (:`then_2`
      ;[1 1 1] Make sure no movement on start
      (set `self.MvtForward` 0.0)
      (set `self.MvtRight` 0.0))))

(fn `UpdateIdle`
  (bind _deltatime (`self.DeltaTime`))
  (`|ExecutionSequence`
    (:`then_0`
      (if (`self.IsMoving`)
        (`/Game/Player/BP_Player.SetState` (`self.PlayerRef`) "NewEnumerator1")
        (`/Game/Player/BP_Player.UpdateHorizontalMovement` (`self.PlayerRef`) (* (`self.MvtForward`) _deltatime) (* (`self.MvtRight`) _deltatime))))
    (:`then_1`
      (`/Game/Player/BP_Player.UpdateAiming` (`self.PlayerRef`) (`self.AimVertical`) (`self.AimHorizontal`)))
    (:`then_2`
      (if (`self.bJumpPressed`)
        (`/Game/Player/BP_Player.DoJump` (`self.PlayerRef`))))))

(fn `UpdateInput`
  (switch `/Game/Player/_Enums/EPlayerState` (`/Game/Player/BP_Player.GetState` (`self.PlayerRef`))
    (:`NewEnumerator0`
      (`self.UpdateIdle`))
    (:`NewEnumerator1`
      (`self.UpdateMoving`))
    (:`NewEnumerator2`
      (`self.UpdateJumping`))))

(fn `UpdateJumping`
  (bind _deltatime (`self.DeltaTime`))
  (`|ExecutionSequence`
    (:`then_0`
      (if (`self.IsOnGround`)
        (`/Game/Player/BP_Player.SetState` (`self.PlayerRef`) "NewEnumerator0")))
    (:`then_1`
      (`/Game/Player/BP_Player.UpdateAiming` (`self.PlayerRef`) (`self.AimVertical`) (`self.AimHorizontal`)))
    (:`then_2`
      (if (`self.IsMoving`)
        (`/Game/Player/BP_Player.UpdateHorizontalMovement` (`self.PlayerRef`) (* (`self.MvtForward`) _deltatime) (* (`self.MvtRight`) _deltatime))))))

(fn `UpdateMoving`
  (bind _deltatime (`self.DeltaTime`))
  (`|ExecutionSequence`
    (:`then_0`
      (if (`self.IsMoving`)
        (`/Game/Player/BP_Player.UpdateHorizontalMovement` (`self.PlayerRef`) (* (`self.MvtForward`) _deltatime) (* (`self.MvtRight`) _deltatime))
        (else
          (`/Game/Player/BP_Player.SetState` (`self.PlayerRef`) "NewEnumerator0"))))
    (:`then_1`
      (`/Game/Player/BP_Player.UpdateAiming` (`self.PlayerRef`) (`self.AimVertical`) (`self.AimHorizontal`)))
    (:`then_2`
      (if (`self.bJumpPressed`)
        (`/Game/Player/BP_Player.DoJump` (`self.PlayerRef`))))))

(fn `UserConstructionScript`)