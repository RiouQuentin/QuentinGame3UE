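; Player character Blueprint exposing movement, sprint, aiming, jump and dash functions, plus health, stamina, key inventory and an enum state.
; InitPlayer resets health, keys and state and sets up the gravity gun component, which receives forwarded grab and throw presses.
; Stamina regenerates on Tick and pays for dashes, which launch along the camera forward and ignore a custom collision channel for one second.
; Damage changes state when health runs out.
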(event `self.ReceiveTick`
  (params (DeltaSeconds :type "Float (single-precision)"))
  (`self.AddStamina` (* (`self.StaminaRegenRate`) DeltaSeconds)))

(event `/Game/Interfaces/IDestructible.TakeDamage`
  (params (Dmage :type "Float (single-precision)"))
  (`self.TakeDamage_Internal` Dmage))

(event `EventDash`
  (`KismetSystemLibrary.Delay` 1.0)
  (`PrimitiveComponent.SetCollisionResponseToChannel` (`self.CapsuleComponent`) "ECC_GameTraceChannel3" "ECR_Block"))

(fn `AddHealth`
  (params (Health :type "Float (double-precision)"))
  (set `self.HealthCurrent` (`KismetMathLibrary.FClamp` (+ (`self.HealthCurrent`) Health) 0.0 (`self.HEalthMax`)))
  (`KismetSystemLibrary.PrintString` (`KismetStringLibrary.Concat_StrStr` "" (`KismetStringLibrary.Conv_DoubleToString` (`self.Get Health`)))))

(fn `AddKeys`
  (params (NbKeys :type Integer))
  (if (> NbKeys 0)
    (set `self.NbKeysCurrent` (+ NbKeys (`self.NbKeysCurrent`)))
    (else
      (`KismetSystemLibrary.PrintString` (`KismetStringLibrary.Concat_StrStr` "Je peut pas ajouter " (`KismetStringLibrary.Conv_IntToString` NbKeys) "Keys")))))

(fn `AddStamina`
  (params (Stamina :type "Float (double-precision)" :default 0.0))
  (set `self.StaminaCurrent` (`KismetMathLibrary.FClamp` (+ (`self.StaminaCurrent`) Stamina) 0.0 (`self.StaminaMax`))))

(fn `Debug`
  (`self.TakeDamage_Internal` 20.0))

(fn `DoDash`
  (if (>= (`self.StaminaCurrent`) (`self.DashCost`))
    (`PrimitiveComponent.SetCollisionResponseToChannel` (`self.CapsuleComponent`) "ECC_GameTraceChannel3" "ECR_Ignore")
    (set `MovementComponent.Velocity` (0.0 0.0 0.0) (`self.CharacterMovement`))
    (`self.LaunchCharacter` (* (`SceneComponent.GetForwardVector` (`self.Camera`)) (`self.DashForce`)))
    (`self.SetState` "NewEnumerator2")
    (`self.SubstrackStamina` (`self.DashCost`))
    (`self.EventDash`)))

(fn `DoJump`
  (`self.LaunchCharacter` (`KismetMathLibrary.MakeVector` 0.0 0.0 (`self.JumpForce`)))
  (`self.SetState` "NewEnumerator2"))

(fn `Force Transform`
  (params (NewTransform :type "Transform Structure"))
  (`|ExecutionSequence`
    (:`then_0`
      (`self.K2_SetActorLocation` (+ (.location NewTransform) (* (`SceneComponent.RelativeLocation` (`self.Body`)) -1.0))))
    (:`then_1`
      (`Controller.SetControlRotation` (`self.GetController`) (.rotation NewTransform)))))

(fn `Get Health`
  (returns (CurrentHealth :type "Float (double-precision)"))
  (return (`self.HealthCurrent`)))

(fn `GetGrabSocket`
  (returns (GrabLocation :type "SceneComponent Object Reference"))
  (return (`self.GravityGrabSocket`)))

(fn `GetStamina`
  (returns (CurrentStamina :type "Float (double-precision)"))
  (return (`self.StaminaCurrent`)))

(fn `GetState`
  (returns (CurrentState :type "/Game/Player/_Enums/EPlayerState Enum"))
  (return (`self.StateCurrent`)))

(fn `HasKey`
  (returns (bHasKey :type Boolean))
  (return (> (`self.NbKeysCurrent`) 0)))

(fn `InitPlayer`
  (`|ExecutionSequence`
    (:`then_0`
      (`/Game/Player/BPC_GravityGun.InitGravityGun` (`self.BPC_GravityGun`) self))
    (:`then_1`
      (set `self.HealthCurrent` (`self.HEalthMax`)))
    (:`then_2`
      (set `self.NbKeysCurrent` 0))
    (:`then_3`
      (`self.SetState` "NewEnumerator0"))))

(fn `OnGravityGrabPressed`
  (`/Game/Player/BPC_GravityGun.OnGrabPressed` (`self.BPC_GravityGun`)))

(fn `OnGravityThrowPressed`
  (`/Game/Player/BPC_GravityGun.OnThrowPressed` (`self.BPC_GravityGun`)))

(fn `RemoveKeys`
  (params (NbKeys :type Integer))
  (bind _returnvalue (- (`self.NbKeysCurrent`) NbKeys))
  (if (> NbKeys 0)
    (if (>= _returnvalue 0)
      (set `self.NbKeysCurrent` _returnvalue))
    (else
      (`KismetSystemLibrary.PrintString` (`KismetStringLibrary.Concat_StrStr` "Je ne peut pas supprimer " (`KismetStringLibrary.Conv_IntToString` NbKeys) "Key")))))

(fn `SetState`
  (params (NewState :type "/Game/Player/_Enums/EPlayerState Enum" :default "NewEnumerator0"))
  (bind _output_get (set `self.StateCurrent` NewState))
  (`KismetSystemLibrary.PrintString` (`KismetStringLibrary.Concat_StrStr` "[Player] NewState=" (`|GetEnumeratorNameAsString` _output_get))))

(fn `SubstrackStamina`
  (params (Stamina :type "Float (double-precision)" :default 0.0))
  (locals (NewLocalVar_0 :type "Float (double-precision)" :default 0.0))
  (set `self.StaminaCurrent` (`KismetMathLibrary.FClamp` (- (`self.StaminaCurrent`) Stamina) 0.0 (`self.StaminaMax`)))
  (`KismetSystemLibrary.PrintString` (`KismetStringLibrary.Concat_StrStr` "" (`KismetStringLibrary.Conv_DoubleToString` (`self.GetStamina`)))))

(fn `TakeDamage_Internal`
  (params (Health :type "Float (double-precision)"))
  (bind _output_get (set `self.HealthCurrent` (- (`self.HealthCurrent`) Health)))
  (if (<= _output_get 0.0)
    (`self.SetState` "NewEnumerator3")
    (else
      (`KismetSystemLibrary.PrintString` (`KismetStringLibrary.Concat_StrStr` "" (`KismetStringLibrary.Conv_DoubleToString` (`self.Get Health`)))))))

(fn `UpdateAiming`
  (params (RotationVertical :type "Float (double-precision)") (RotationHorizontal :type "Float (double-precision)"))
  (locals (L_rotVertical :type "Float (double-precision)") (L_rotHorizontal :type "Float (double-precision)"))
  (bind _returnvalue (`self.GetController`))
  (bind (_returnvalue_roll _returnvalue_pitch _returnvalue_yaw) (`KismetMathLibrary.BreakRotator` (`Controller.GetControlRotation` _returnvalue)))
  (`|ExecutionSequence`
    (:`then_0`
      (set `local.L_rotVertical` (* RotationVertical (`self.AimSpeedVertical`))))
    (:`then_1`
      (set `local.L_rotHorizontal` (* RotationHorizontal (`self.AimSpeedHorizontal`))))
    (:`then_2`
      (`Controller.SetControlRotation` _returnvalue (`KismetMathLibrary.MakeRotator` 0.0 (+ _returnvalue_pitch (`local.L_rotVertical`)) (+ _returnvalue_yaw (`local.L_rotHorizontal`)))))))

(fn `UpdateHorizontalMovement`
  (params (MvtForward :type "Float (double-precision)") (MvtRight :type "Float (double-precision)") (IsSprint :type Boolean))
  (bind _returnvalue (select `bool` IsSprint :`false` (`self.MvtSpeedForward`) :`true` (`self.SprintSpeed`)))
  (`|ExecutionSequence`
    (:`then_0`
      (set `CharacterMovementComponent.MaxWalkSpeed` _returnvalue (`self.CharacterMovement`))
      (`self.AddMovementInput` (`self.GetActorForwardVector`) (* MvtForward _returnvalue)))
    (:`then_1`
      (`self.AddMovementInput` (`self.GetActorRightVector`) (* MvtRight (`self.MvtSpeedRight`))))))

(fn `UserConstructionScript`)