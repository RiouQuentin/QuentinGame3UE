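; Player component that implements a gravity gun for grabbing, dropping and throwing BP_GravityTargetBase actors.
; Every tick, a debug-drawn line trace from the player's camera records the gravity target in sight.
; Grab toggles between attaching that target to the player's grab socket and dropping the held one, while throw launches it along the camera's forward vector.
; The target itself handles each action through its OnGrabbed, OnDropped and OnThrown functions.
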(event `self.ReceiveTick`
  (params (DeltaSeconds :type "Float (single-precision)"))
  (`self.UpdateTarget`))

(fn `InitGravityGun`
  (params (PlayerRef :type "/Game/Player/BP_Player Object Reference"))
  (`|ExecutionSequence`
    (:`then_0`
      (set `self.PlayerRef` PlayerRef))
    (:`then_1`
      (set `self.GravityTargetCurrent` null))
    (:`then_2`
      (set `self.GravityTargetInsight` null))))

(fn `OnGrabPressed`
  (bind _gravitytargetcurrent (`self.GravityTargetCurrent`)
    (:`then`
      (`/Game/LDIs/GravityTargets/_Base/BP_GravityTargetBase.OnDropped` _gravitytargetcurrent)
      (set `self.GravityTargetCurrent` null))
    (:`else`
      (bind _gravitytargetinsight (`self.GravityTargetInsight`)
        (:`then`
          (bind _output_get (set `self.GravityTargetCurrent` _gravitytargetinsight))
          (`/Game/LDIs/GravityTargets/_Base/BP_GravityTargetBase.OnGrabbed` _output_get (`/Game/Player/BP_Player.GetGrabSocket` (`self.PlayerRef`))))
        (:`else`)))))

(fn `OnThrowPressed`
  (bind _gravitytargetcurrent (`self.GravityTargetCurrent`)
    (:`then`
      (`/Game/LDIs/GravityTargets/_Base/BP_GravityTargetBase.OnThrown` _gravitytargetcurrent (* (`SceneComponent.GetForwardVector` (`/Game/Player/BP_Player.Camera` (`self.PlayerRef`))) (`self.GravityThrowForce`)))
      (set `self.GravityTargetCurrent` null))
    (:`else`)))

(fn `UpdateTarget`
  (bind _camera (`/Game/Player/BP_Player.Camera` (`self.PlayerRef`)))
  (bind _returnvalue (`SceneComponent.K2_GetComponentLocation` _camera))
  (bind _outhit (`KismetSystemLibrary.LineTraceSingle` :`Start` _returnvalue :`End` (+ _returnvalue (* (`SceneComponent.GetForwardVector` _camera) (`self.LineTraceLenght`))) :`TraceChannel` "TraceTypeQuery3" :`DrawDebugType` "ForOneFrame"))
  (bind (_bblockinghit _binitialoverlap _time _distance _location _impactpoint _normal _impactnormal _physmat _hitactor) (`GameplayStatics.BreakHitResult` _outhit))
  (if _bblockinghit
    (bind _asbp_gravity_target_base (cast `/Game/LDIs/GravityTargets/_Base/BP_GravityTargetBase` _hitactor)
      (:`then`
        (set `self.GravityTargetInsight` _asbp_gravity_target_base))
      (:`CastFailed`
        (set `self.GravityTargetInsight` null :!label _label)))
    (else
      (goto _label))))