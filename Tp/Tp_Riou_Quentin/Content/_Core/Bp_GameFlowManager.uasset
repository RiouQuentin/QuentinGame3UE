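; Game flow manager that runs the session's state machine across loading, gameplay, game over and level complete, tracking playtime.
; On BeginPlay it caches the player and controller, creates the flow UI and streams the first entry of its level array as a level instance.
; State changes drive UI and input mode; PerformNextStep reloads, advances or quits after the last level.
; OnLevelEnd currently ignores IsComplete and always sets LevelComplete.
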(event `self.ReceiveBeginPlay`
  (`self.InitGameManager`))

(event `self.ReceiveTick`
  (params (DeltaSeconds :type "Float (single-precision)"))
  (if (`|EnumEquality` (`self.StateCurrent`) "NewEnumerator1")
    (set `self.Playtime` (+ DeltaSeconds (`self.Playtime`)))))

(fn `InitGameManager`
  (bind _gameflowuiref (`self.GameFlowUIRef`))
  (`|ExecutionSequence`
    (:`then_0`
      (`self.PlayerRef`
        (:`then`)
        (:`else`
          (bind _outactors (`GameplayStatics.GetAllActorsOfClass` "/Game/Player/BP_Player.BP_Player_C"))
          (bind _output_get (set `self.PlayerRef` (`|GetArrayItem` _outactors)))
          (bind _asbp_player_controller (cast `/Game/Player/BP_PlayerController` (`Pawn.GetController` _output_get)))
          (set `self.PlayerControllerRef` _asbp_player_controller))))
    (:`then_1`
      (`self.GameFlowUIRef`
        (:`then`)
        (:`else`
          (bind _returnvalue (`|CreateWidget` "/Game/_Core/_Widget/WBP_GameFlowUI.WBP_GameFlowUI_C" (`self.PlayerControllerRef`)))
          (set `self.GameFlowUIRef` _returnvalue)
          (`|ExecutionSequence`
            (:`then_0`
              (`/Game/_Core/_Widget/WBP_GameFlowUI.InitWidget` _gameflowuiref self (`self.PlayerRef`)))
            (:`then_1`
              (`UserWidget.AddToViewport` _gameflowuiref 0))))))
    (:`then_2`
      (set `self.Playtime` 0.0))
    (:`then_3`
      (set `self.CurrentLevelIndex ` 0))
    (:`then_4`
      (`self.LoadLevel` (`self.CurrentLevelIndex `)))))

(fn `IsLastLevel`
  (returns (bLastLevel :type Boolean))
  (return (== (- (`KismetArrayLibrary.Array_Length` (`self.Level`)) 1) (`self.CurrentLevelIndex `))))

(fn `LoadLevel`
  (params (LevelIdex :type Integer))
  (`|ExecutionSequence`
    (:`then_0`
      (set `self.Playtime` 0.0))
    (:`then_1`
      (`self.SetState` "NewEnumerator4"))
    (:`then_2`
      (bind (_boutsuccess _returnvalue) (`LevelStreamingDynamic.LoadLevelInstanceBySoftObjectPtr` (`|GetArrayItem` (`self.Level`) LevelIdex) (0.0 0.0 0.0) (struct) "" null))
      (bind _output_get (set `self.CurrentLevel ` _returnvalue))
      (add `LevelStreaming.OnLevelLoaded` _output_get (`|CreateDelegate` :!event `OnLevelLoaded`)))))

(fn `OnGameOver`
  (`|ExecutionSequence`
    (:`then_0`
      (`/Game/_Core/_Widget/WBP_GameFlowUI.OnGameplayEnd` (`self.GameFlowUIRef`) true (`self.Playtime`)))
    (:`then_1`
      (`self.ShowMouseCursor` true))))

(fn `OnGameplay`
  (`|ExecutionSequence`
    (:`then_0`
      (`/Game/_Core/_Widget/WBP_GameFlowUI.OnGameplay` (`self.GameFlowUIRef`)))
    (:`then_1`
      (`self.ShowMouseCursor` false))))

(fn `OnLevelComplete`
  (`|ExecutionSequence`
    (:`then_0`
      (`/Game/_Core/_Widget/WBP_GameFlowUI.OnGameplayEnd` (`self.GameFlowUIRef`) false (`self.Playtime`)))
    (:`then_1`
      (`self.ShowMouseCursor` false))
    (:`then_2`
      (`self.UnloadCurrentLevel`))))

(fn `OnLevelEnd`
  (params (bIsComplete :type Boolean))
  (if true
    (`self.SetState` "NewEnumerator3")
    (else
      (`self.SetState` "NewEnumerator2"))))

(fn `OnLevelLoaded`
  (`self.SetState` "NewEnumerator1"))

(fn `OnLoadingLevel`
  (`/Game/_Core/_Widget/WBP_GameFlowUI.OnLoadingLevel` (`self.GameFlowUIRef`)))

(fn `PerformNextStep`
  (if (`|EnumEquality` (`self.StateCurrent`) "NewEnumerator2")
    (`self.ReloadLevel`)
    (elif (`self.IsLastLevel`)
      (`KismetSystemLibrary.QuitGame` null "Quit")
      (else
        (bind _result (`/Engine/EditorBlueprintResources/StandardMacros.IncrementInt` (`self.CurrentLevelIndex `))
          (:`  `
            (`self.LoadLevel` _result)))))))

(fn `ReloadLevel`
  (`|ExecutionSequence`
    (:`then_0`
      (`self.UnloadCurrentLevel`))
    (:`then_1`
      (`self.LoadLevel` (`self.CurrentLevelIndex `)))))

(fn `RespawnPlayer`
  (bind _playerref (`self.PlayerRef`))
  (`|ExecutionSequence`
    (:`then_0`
      (`/Game/Player/BP_Player.InitPlayer` _playerref))
    (:`then_1`
      (`/Game/Player/BP_Player.Force Transform` _playerref (`self.GetTransform` (`self.CurrentStartPos`))))))

(fn `SetStartPosition`
  (params (StartPosition :type "/Game/_Core/Bp_StartPosition Object Reference"))
  (set `self.CurrentStartPos` StartPosition)
  (`|ExecutionSequence`
    (:`then_0`
      (`self.RespawnPlayer`))
    (:`then_1`
      (`self.SetState` "NewEnumerator1"))))

(fn `SetState`
  (params (NewState :type "/Game/_Core/_Enums/EGameState Enum" :default "NewEnumerator0"))
  (bind _output_get (set `self.StateCurrent` NewState))
  (switch `/Game/_Core/_Enums/EGameState` _output_get
    (:`NewEnumerator1`
      (`self.OnGameplay`))
    (:`NewEnumerator2`
      (`self.OnGameOver`))
    (:`NewEnumerator3`
      (`self.OnLevelComplete`))
    (:`NewEnumerator4`
      (`self.OnLoadingLevel`))))

(fn `ShowMouseCursor`
  (params (bShow :type Boolean))
  (bind _playercontrollerref (`self.PlayerControllerRef`))
  (bind _playercontrollerref_2 (`self.PlayerControllerRef`))
  (if bShow
    (`WidgetBlueprintLibrary.SetInputMode_UIOnlyEx` _playercontrollerref (`self.GameFlowUIRef`) "LockAlways")
    (set `PlayerController.bShowMouseCursor` true _playercontrollerref)
    (else
      (`WidgetBlueprintLibrary.SetInputMode_GameOnly` _playercontrollerref_2)
      (set `PlayerController.bShowMouseCursor` false _playercontrollerref_2))))

(fn `UnloadCurrentLevel`
  (`LevelStreaming.SetIsRequestingUnloadAndRemoval` (`self.CurrentLevel `) true))

(fn `UserConstructionScript`
  (set `self.StateCurrent` "NewEnumerator0"))